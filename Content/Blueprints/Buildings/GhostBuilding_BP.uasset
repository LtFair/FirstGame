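; GhostBuilding_BP is a ghost building that holds a pending building's display mesh, building class and construction proxy.
; OnSpawn stores these and applies the mesh to GhostBuildingMesh, ignoring calls while the ghost is already active.
; KillGhost clears the stored references and active flag for reuse, but does not clear the mesh component or destroy the actor.
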(event `On Spawn`
  (params (`Display Mesh` :type "StaticMesh Object Reference") (`Building Class` :type "/Game/Blueprints/Buildings/BuildingMaster_BP Class Reference") (`Construction Proxy` :type "/Game/Blueprints/Construction/ConstructionProxy_BP Class Reference"))
  (if (not (`self.IsActive`))
    (set `self.Building Class` `Building Class`)
    (set `self.ConstructionProxy` `Construction Proxy`)
    (bind _output_get (set `self.DisplayMesh` `Display Mesh`))
    (set `self.IsActive` true)
    (`StaticMeshComponent.SetStaticMesh` (`self.GhostBuilding_Mesh`) _output_get)))

(event `Kill Ghost`
  (set `self.Building Class` null)
  (set `self.ConstructionProxy` null)
  (set `self.DisplayMesh` null)
  (set `self.IsActive` false))

(fn `UserConstructionScript`)