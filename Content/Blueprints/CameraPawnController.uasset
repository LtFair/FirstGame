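; Player controller for a top-down building game, driving the CameraPawn and setting up the cursor, main HUD and ghost building actor on begin play.
; Axis input and screen-edge scrolling move the pawn, with Shift boosting both and key movement also scaling with spring-arm zoom.
; Holding Pan opens gates for mouse rotation with clamped pitch and suspends navigation.
; BuildBuilding, clock and calendar functions are stubs, and the construction manager spawn is unconnected.
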(event `self.ReceiveBeginPlay`
  ;[1 1 1] Begin Play
  (`|ExecutionSequence`
    (:`then_0`
      (`self.ReferenceCasts`))
    (:`then_1`
      (`WidgetBlueprintLibrary.SetInputMode_GameAndUIEx` self null "LockAlways" false)
      (set `self.bShowMouseCursor` true)
      (`self.Create HUDs`)
      (`UserWidget.AddToViewport` (`self.Main UI HUD`) 0))
    (:`then_3`
      (bind _returnvalue (`|SpawnActorFromClass` "/Game/Blueprints/Buildings/GhostBuilding_BP.GhostBuilding_BP_C" (`KismetMathLibrary.MakeTransform` (0.0 0.0 0.0)) "AlwaysSpawn" "OverrideRootScale" null self null))
      (set `self.Ghost Building Ref` _returnvalue))))

(event `InputAxis|Move Forward`
  (params (AxisValue :type "Float (single-precision)"))
  (bind _camerapawnref (`self.CameraPawnRef`))
  ;[1 1 1] Camera Movement
  ;;[1 1 1] Controls movement in the X direction (north and south)
  (if (not (`self.DisableCamNav`))
    (`self.K2_SetActorTransform` _camerapawnref (`self.MovementX` (`self.MovementSpeedCalc`) (`self.FastMoveMultiplier`) AxisValue _camerapawnref) false false)))

(event `InputAxis|Move side`
  (params (AxisValue :type "Float (single-precision)"))
  (bind _camerapawnref (`self.CameraPawnRef`))
  ;[1 1 1] Camera Movement
  ;;[1 1 1] Controls movement in the Y direction (right and left)
  (if (not (`self.DisableCamNav`))
    (`self.K2_SetActorTransform` _camerapawnref (`KismetMathLibrary.MakeTransform` (`KismetMathLibrary.MakeVector` (.x (.location (`self.MovementY` (`self.MovementSpeedCalc`) (`self.FastMoveMultiplier`) AxisValue _camerapawnref))) (.y (.location (`self.MovementY` (`self.MovementSpeedCalc`) (`self.FastMoveMultiplier`) AxisValue _camerapawnref))) 100.0) (.rotation (`self.MovementY` (`self.MovementSpeedCalc`) (`self.FastMoveMultiplier`) AxisValue _camerapawnref)) (.scale (`self.MovementY` (`self.MovementSpeedCalc`) (`self.FastMoveMultiplier`) AxisValue _camerapawnref))) false false)))

(event `Key|LeftShift`
  (params (Key :type "Key Structure"))
  ;[1 1 1] Camera Movement
  ;;[1 1 1] Move multiplier
  (:`Pressed`
    (set `self.FastMoveMultiplier` 2.0))
  (:`Released`
    (set `self.FastMoveMultiplier` 1.0)))

(event `InputAction|Zoom In`
  (params (Key :type "Key Structure"))
  (bind _springarm (`/Game/Blueprints/CameraPawn.SpringArm` (`self.CameraPawnRef`)))
  ;[1 1 1] Camera Movement
  ;;[1 1 1] Zoom Camera In
  (:`Pressed`
    (set `SpringArmComponent.TargetArmLength` (`KismetMathLibrary.FClamp` (- (`SpringArmComponent.TargetArmLength` _springarm) 100.0) 500.0 1500.0) _springarm)))

(event `InputAction|Zoom Out`
  (params (Key :type "Key Structure"))
  (bind _springarm (`/Game/Blueprints/CameraPawn.SpringArm` (`self.CameraPawnRef`)))
  ;[1 1 1] Camera Movement
  ;;[1 1 1] Zoom Camera Out
  (:`Pressed`
    (set `SpringArmComponent.TargetArmLength` (`KismetMathLibrary.FClamp` (+ (`SpringArmComponent.TargetArmLength` _springarm) 100.0) 500.0 1500.0) _springarm)))

(event `InputAction|Pan Reset`
  (params (Key :type "Key Structure"))
  (bind _camerapawnref (`self.CameraPawnRef`))
  ;[1 1 1] Camera Movement
  ;;[1 1 1] Pan Reset
  (:`Pressed`
    (`self.K2_SetActorRotation` _camerapawnref (`KismetMathLibrary.MakeRotator` (.roll (`self.K2_GetActorRotation` _camerapawnref)) 0.0 (.yaw (`self.K2_GetActorRotation` _camerapawnref))) false)))

(event `InputAxisKey|MouseX`
  (params (AxisValue :type "Float (single-precision)"))
  (bind _camerapawnref (`self.CameraPawnRef`))
  ;[1 1 1] Camera Movement
  ;;[1 1 1] Pan X
  (`/Engine/EditorBlueprintResources/StandardMacros.Gate` true :!label _label
    (:`Exit`
      (`self.K2_SetActorRotation` _camerapawnref (`KismetMathLibrary.MakeRotator` (.roll (`self.K2_GetActorRotation` _camerapawnref)) (.pitch (`self.K2_GetActorRotation` _camerapawnref)) (+ (.yaw (`self.K2_GetActorRotation` _camerapawnref)) (* (`self.PanSensativity`) AxisValue))) false))))

(event `InputAxisKey|MouseY`
  (params (AxisValue :type "Float (single-precision)"))
  (bind _camerapawnref (`self.CameraPawnRef`))
  ;[1 1 1] Camera Movement
  ;;[1 1 1] Pan Y
  (`/Engine/EditorBlueprintResources/StandardMacros.Gate` true :!label _label_2
    (:`Exit`
      (`self.K2_SetActorRotation` _camerapawnref (`KismetMathLibrary.MakeRotator` (.roll (`self.K2_GetActorRotation` _camerapawnref)) (`KismetMathLibrary.FClamp` (+ (.pitch (`self.K2_GetActorRotation` _camerapawnref)) (* (`self.PanSensativity`) AxisValue)) -15.0 60.0) (.yaw (`self.K2_GetActorRotation` _camerapawnref))) false))))

(event `InputAction|Pan`
  (params (Key :type "Key Structure"))
  ;[1 1 1] Camera Movement
  ;;[1 1 1] Pan Y
  (:`Pressed`
    (set `self.DisableCamNav` true)
    (goto _label_2 :!via `Open`))
  (:`Released`
    (set `self.DisableCamNav` false)
    (goto _label_2 :!via `Close`)))

(event `InputAction|Pan`
  (params (Key :type "Key Structure"))
  ;[1 1 1] Camera Movement
  ;;[1 1 1] Pan X
  (:`Pressed`
    (set `self.DisableCamNav` true)
    (goto _label :!via `Open`))
  (:`Released`
    (set `self.DisableCamNav` false)
    (goto _label :!via `Close`)))

(event `InputAxisKey|MouseX`
  (params (AxisValue :type "Float (single-precision)"))
  ;[1 1 1] Camera Movement
  ;;[1 1 1] Mouse Edge Movement
  (if (not (`self.DisableCamNav`))
    (bind (_delta_x_speed _delta_y_speed) (`self.ScreenEdgeMovement` :!label _label_3))
    (`self.K2_AddActorLocalOffset` (`self.CameraPawnRef`) (`KismetMathLibrary.MakeVector` _delta_x_speed _delta_y_speed) true false)))

(event `InputAxisKey|MouseY`
  (params (AxisValue :type "Float (single-precision)"))
  ;[1 1 1] Camera Movement
  ;;[1 1 1] Mouse Edge Movement
  (if (not (`self.DisableCamNav`))
    (goto _label_3 :!via `Mouse Y`)))

(event `/Game/Interfaces/I_HUD.Build Building`
  (params (MainBuilding :type "/Game/Blueprints/Buildings/BuildingMaster_BP Class Reference")))

(fn `MovementSpeedCalc`
  (returns (MoveSensativity :type "Float (double-precision)"))
  ;[1 1 1] Determines the camera pan speed based on how zoomed in the user is
  (return (`KismetMathLibrary.FClamp` (/ (`SpringArmComponent.TargetArmLength` (`/Game/Blueprints/CameraPawn.SpringArm` (`self.CameraPawnRef`))) 100.0) 5.0 20.0)))

(fn `Set Calendar`
  (params (Date :type "Array of Integer (by ref)"))
  (returns (Success :type Boolean))
  (return false))

(fn `Set Clock`
  (params (Time :type "Array of Integer (by ref)"))
  (returns (Success :type Boolean))
  (return false))

(fn `UserConstructionScript`)